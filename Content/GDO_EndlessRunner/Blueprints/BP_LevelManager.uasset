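; BP_LevelManager builds the endless road for a runner along the world X axis.
; At BeginPlay it spawns ten BP_RoadTile actors end to end, advancing NextTileX by TileLength for each.
; Every Tick it checks whether the player character is over 1500 units past the oldest tile.
; If so, it teleports that tile to the front and requeues it in ActiveTiles, reusing actors instead of respawning.
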(event `self.ReceiveBeginPlay`
  (for _ (range 10)
    (`self.SpawnNextTile`)))

(event `self.ReceiveTick`
  (params (DeltaSeconds :type "Float (single-precision)"))
  (bind _returnvalue (`GameplayStatics.GetPlayerCharacter` 0))
  (bind _activetiles (`self.ActiveTiles`))
  (bind _returnvalue_x (`KismetMathLibrary.BreakVector` (`self.K2_GetActorLocation` _returnvalue)))
  (bind _output (`|GetArrayItem` _activetiles))
  (bind _returnvalue_x_2 (`KismetMathLibrary.BreakVector` (`self.K2_GetActorLocation` _output)))
  (if (`KismetArrayLibrary.Array_IsValidIndex` _activetiles)
    (`/Engine/EditorBlueprintResources/StandardMacros.IsValid` _output
      (:`Is Valid`
        (`/Engine/EditorBlueprintResources/StandardMacros.IsValid` _returnvalue
          (:`Is Valid`
            (if (< (+ _returnvalue_x_2 1500.0) _returnvalue_x)
              (`self.RecycleOldestTile`))))))))

(fn `RecycleOldestTile`
  (locals (OldTile :type "/Game/GDO_EndlessRunner/Blueprints/BP_RoadTile Object Reference"))
  (bind _activetiles (`self.ActiveTiles`))
  (bind _nexttilex (`self.NextTileX`))
  (bind _output_get (set `local.OldTile` (`|GetArrayItem` _activetiles)))
  (`self.K2_SetActorLocation` _output_get (`KismetMathLibrary.MakeVector` _nexttilex) false true)
  (`KismetArrayLibrary.Array_Remove` _activetiles)
  (`KismetArrayLibrary.Array_Add` _activetiles _output_get)
  (set `self.NextTileX` (+ _nexttilex (`self.TileLength`))))

(fn `SpawnNextTile`
  (bind _nexttilex (`self.NextTileX`))
  (bind _returnvalue (`|SpawnActorFromClass` "/Game/GDO_EndlessRunner/Blueprints/BP_RoadTile.BP_RoadTile_C" (`KismetMathLibrary.MakeTransform` (`KismetMathLibrary.MakeVector` _nexttilex)) "AlwaysSpawn" "MultiplyWithRoot" null null))
  (`KismetArrayLibrary.Array_Add` (`self.ActiveTiles`) _returnvalue)
  (set `self.NextTileX` (+ _nexttilex (`self.TileLength`))))

(fn `UserConstructionScript`)