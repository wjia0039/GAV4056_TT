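; BP_RoadTile is a recycled road segment for an endless runner, carrying enemies and pickups.
; On Tick, once the player is over 1500 units ahead along X, it teleports 10000 units forward and calls RefreshLayout, which also runs at BeginPlay.
; RefreshLayout randomizes PatrolEnemy along X and puts RobotEnemy and the score, shield and speed pickups in random lanes (three possible).
; Only the score orb has its collision and visibility restored.
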(event `self.ReceiveBeginPlay`
  (`self.RefreshLayout`))

(event `self.ReceiveTick`
  (params (DeltaSeconds :type "Float (single-precision)"))
  (bind _returnvalue_x (`KismetMathLibrary.BreakVector` (`self.K2_GetActorLocation`)))
  (bind _returnvalue_x_2 (`KismetMathLibrary.BreakVector` (`self.K2_GetActorLocation` (`GameplayStatics.GetPlayerCharacter` 0))))
  (if (> (- _returnvalue_x_2 _returnvalue_x) 1500.0)
    (`self.K2_AddActorWorldOffset` (10000.0 0.0 0.0) false true)
    (`self.RefreshLayout`)))

(fn `RefreshLayout`
  (bind _scoreorb (`self.ScoreOrb`))
  (bind _returnvalue (* (`KismetMathLibrary.RandomIntegerInRange` -1 1) 400))
  (bind _childactor (`ChildActorComponent.ChildActor` _scoreorb))
  (bind _returnvalue_2 (`KismetMathLibrary.Conv_IntToDouble` _returnvalue))
  (`SceneComponent.K2_SetRelativeLocation` (`self.PatrolEnemy`) (`KismetMathLibrary.MakeVector` (`KismetMathLibrary.RandomFloatInRange` -350.0 -150.0) 0.0 90.0) false false)
  (`SceneComponent.K2_SetRelativeLocation` _scoreorb (`KismetMathLibrary.MakeVector` 450.0 (`KismetMathLibrary.Conv_IntToDouble` _returnvalue) 60.0) false false)
  (`self.SetActorEnableCollision` _childactor true)
  (`self.SetActorHiddenInGame` _childactor false)
  (`SceneComponent.K2_SetRelativeLocation` (`self.ShieldPickup`) (`KismetMathLibrary.MakeVector` -450.0 _returnvalue_2 60.0) false false)
  (`SceneComponent.K2_SetRelativeLocation` (`self.SpeedPickup`) (`KismetMathLibrary.MakeVector` -50.0 _returnvalue_2 60.0) false false)
  (`SceneComponent.K2_SetRelativeLocation` (`self.RobotEnemy`) (`KismetMathLibrary.MakeVector` 250.0 _returnvalue_2 90.0) false false))

(fn `UserConstructionScript`)