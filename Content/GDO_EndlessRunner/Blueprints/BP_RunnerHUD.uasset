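; Endless runner HUD that draws health and score plus a paused main or game-over menu.
; DrawHUD shows the menu when the "Playing" level option is absent or health reaches zero.
; Canvas hit boxes serve as buttons that reload the level with or without that option, or quit.
; The best score loads at BeginPlay and is saved to a slot whenever the menu draws a higher one.
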(event `self.ReceiveBeginPlay`
  (bind _returnvalue (`GameplayStatics.LoadGameFromSlot` "RunnerBest"))
  (bind _asbp_runner_save (cast `/Game/GDO_EndlessRunner/Blueprints/BP_RunnerSave` _returnvalue))
  (set `self.BestScore` (`/Game/GDO_EndlessRunner/Blueprints/BP_RunnerSave.BestScore` _asbp_runner_save)))

(event `self.ReceiveDrawHUD`
  (params (SizeX :type Integer) (SizeY :type Integer))
  (bind _asbp_runner_character (cast `/Game/GDO_EndlessRunner/Blueprints/BP_RunnerCharacter` (`self.GetOwningPawn`)))
  (bind _health (`/Game/GDO_EndlessRunner/Blueprints/BP_RunnerCharacter.Health` _asbp_runner_character))
  (bind _score (`/Game/GDO_EndlessRunner/Blueprints/BP_RunnerCharacter.Score` _asbp_runner_character))
  (`self.DrawText` (`KismetStringLibrary.Concat_StrStr` "HP: " (`KismetStringLibrary.Conv_DoubleToString` _health) "    Points: " (`KismetStringLibrary.Conv_IntToString` _score)) (struct :`A` 1) 40.0 40.0 null 3.0)
  (if (`GameplayStatics.HasOption` (`GameModeBase.OptionsString` (`GameplayStatics.GetGameMode`)) "Playing")
    (bind _returnvalue (<= _health 0.0))
    (if _returnvalue
      (`self.DrawMenu` _returnvalue _score :!label _label))
    (else
      (goto _label))))

(event `self.ReceiveHitBoxClick`
  (params (BoxName :type Name))
  (switch `name` BoxName
    (:`Primary`
      (`GameplayStatics.OpenLevel` "LV_EndlessRunner" true "Playing"))
    (:`Secondary`
      (if (<= (`/Game/GDO_EndlessRunner/Blueprints/BP_RunnerCharacter.Health` (stale `self.ReceiveDrawHUD` _asbp_runner_character)) 0.0)
        (`GameplayStatics.OpenLevel` "LV_EndlessRunner")
        (else
          (`KismetSystemLibrary.QuitGame` null "Quit"))))))

(fn `DrawMenu`
  (params (IsDead :type Boolean) (RoundScore :type Integer))
  (bind _returnvalue (`self.GetOwningPlayerController`))
  (`self.DrawRect` (struct :`R` 0.871367 :`G` 0.904661 :`B` 0.938686 :`A` 0.94902) 80.0 120.0 600.0 400.0)
  (`self.DrawText` (`KismetMathLibrary.SelectString` "GAME OVER \n \n[ Restart ] \n \n[ Main Menu ]" "ENDLESS RUNNER \n \n[ Play ] \n \n[ Exit ]" IsDead) (struct :`A` 1) 120.0 160.0 null 3.0)
  (`self.AddHitBox` (100.0 220.0) (450.0 65.0) "Primary" true)
  (`self.AddHitBox` (100.0 300.0) (450.0 65.0) "Secondary" true)
  (set `PlayerController.bShowMouseCursor` true _returnvalue)
  (`GameplayStatics.SetGamePaused` true)
  (set `PlayerController.bEnableClickEvents` true _returnvalue)
  (`self.SaveBestScore` RoundScore)
  (`self.DrawText` (`KismetStringLibrary.Concat_StrStr` "This run: " (`KismetStringLibrary.Conv_IntToString` RoundScore) "    Best: " (`KismetStringLibrary.Conv_IntToString` (`self.BestScore`))) (struct :`A` 1) 120.0 420.0 null 2.0))

(fn `SaveBestScore`
  (params (RoundScore :type Integer))
  (if (> RoundScore (`self.BestScore`))
    (set `self.BestScore` RoundScore)
    (bind _returnvalue (`GameplayStatics.CreateSaveGameObject` "/Game/GDO_EndlessRunner/Blueprints/BP_RunnerSave.BP_RunnerSave_C"))
    (set `/Game/GDO_EndlessRunner/Blueprints/BP_RunnerSave.BestScore` RoundScore _returnvalue)
    (`GameplayStatics.SaveGameToSlot` _returnvalue "RunnerBest")))

(fn `UserConstructionScript`)